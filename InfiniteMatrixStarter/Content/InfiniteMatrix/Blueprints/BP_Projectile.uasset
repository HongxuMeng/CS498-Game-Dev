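; BP_Projectile is a projectile actor that flies along world X and destroys itself on hit or timeout.
; On BeginPlay it derives its speed from the player's current ForwardSpeed, and its lifetime from that speed relative to the player's initial speed.
; Tick counts down the lifetime and moves the actor with a swept offset.
; Hits on the Cone, Cylinder or BoxCollision components destroy it; DestroyProjectile is an empty stub.
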(event `self.ReceiveBeginPlay`
  (bind _asbp_player (cast `/Game/InfiniteMatrix/Blueprints/BP_Player` (`GameplayStatics.GetPlayerPawn` 0)))
  (bind _forwardspeed_ (`/Game/InfiniteMatrix/Blueprints/BP_Player.ForwardSpeed ` _asbp_player))
  (set `self.ForwardSpeed` (* _forwardspeed_ (`self.ProjectileSpeedIndex`)))
  (set `self.TTL` (* (/ _forwardspeed_ (`/Game/InfiniteMatrix/Blueprints/BP_Player.ForwardSpeedInitial` _asbp_player)) (`self.TTLIndex`))))

(event `self.ReceiveTick`
  (params (DeltaSeconds :type "Float (single-precision)"))
  (bind _returnvalue (- (`self.TTL`) DeltaSeconds))
  (set `self.TTL` _returnvalue)
  (if (<= _returnvalue 0.0)
    (`self.K2_DestroyActor`)
    (else
      (`self.K2_AddActorWorldOffset` (`KismetMathLibrary.MakeVector` (* DeltaSeconds (`self.ForwardSpeed`))) true))))

(event `self.Cone.OnComponentHit`
  (params (HitComponent :type "PrimitiveComponent Object Reference") (OtherActor :type "Actor Object Reference") (OtherComp :type "PrimitiveComponent Object Reference") (NormalImpulse :type "Vector Structure") (Hit :type "HitResult Structure (by ref)"))
  (`self.K2_DestroyActor` :!label _label))

(event `self.Cylinder.OnComponentHit`
  (params (HitComponent :type "PrimitiveComponent Object Reference") (OtherActor :type "Actor Object Reference") (OtherComp :type "PrimitiveComponent Object Reference") (NormalImpulse :type "Vector Structure") (Hit :type "HitResult Structure (by ref)"))
  (goto _label))

(event `self.BoxCollision.OnComponentHit`
  (params (HitComponent :type "PrimitiveComponent Object Reference") (OtherActor :type "Actor Object Reference") (OtherComp :type "PrimitiveComponent Object Reference") (NormalImpulse :type "Vector Structure") (Hit :type "HitResult Structure (by ref)"))
  (goto _label))

(fn `DestroyProjectile`)

(fn `UserConstructionScript`)